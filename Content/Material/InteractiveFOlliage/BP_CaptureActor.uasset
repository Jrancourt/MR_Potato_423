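; Scene capture actor for interactive grass that follows the player and records components tagged GrassAffector.
; On BeginPlay it writes the capture's ortho width to MPC_Grass and registers tagged primitive components on tagged actors as show-only, a one-time scan.
; A fast looping timer moves it to the player's XY at fixed height and publishes that location to MPC_Grass, so materials can locate the capture area.
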(event `self.ReceiveBeginPlay`
  (`KismetMaterialLibrary.SetScalarParameterValue` "/Game/Material/InteractiveFOlliage/MPC_Grass.MPC_Grass" "CaptureSize" (`SceneCaptureComponent2D.OrthoWidth` (`self.SceneCaptureComponent2D`)))
  (`KismetSystemLibrary.K2_SetTimer` null "MoveTarget" 0.01 true)
  (bind _outactors (`GameplayStatics.GetAllActorsWithTag` "GrassAffector"))
  (for _array_element _outactors
    (for _array_element_2 (`self.GetComponentsByTag` _array_element "/Script/Engine.PrimitiveComponent" "GrassAffector")
      (`SceneCaptureComponent.ShowOnlyComponent` (`self.SceneCaptureComponent2D`) _array_element_2))))

(event `MoveTarget`
  (bind (_returnvalue_x _returnvalue_y _returnvalue_z) (`KismetMathLibrary.BreakVector` (`self.K2_GetActorLocation`)))
  (bind (_returnvalue_x_2 _returnvalue_y_2) (`KismetMathLibrary.BreakVector` (`self.K2_GetActorLocation` (`GameplayStatics.GetPlayerCharacter` 0))))
  (`self.K2_SetActorLocation` (`KismetMathLibrary.MakeVector` _returnvalue_x_2 _returnvalue_y_2 _returnvalue_z))
  (`KismetMaterialLibrary.SetVectorParameterValue` "/Game/Material/InteractiveFOlliage/MPC_Grass.MPC_Grass" "CaptureLocation" (`KismetMathLibrary.Conv_VectorToLinearColor` (`self.K2_GetActorLocation`))))

(fn `UserConstructionScript`)